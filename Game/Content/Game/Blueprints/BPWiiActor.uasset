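; Aim reticle actor steered by Wii Remote MotionPlus, orbiting the FpsCharacter's first-person camera at a fixed distance.
; The first non-zero readings set a neutral pitch/roll and deadzone thresholds; deviations beyond them become frame-time-scaled movement.
; Each tick it faces the camera, re-projects onto that sphere and applies a local offset; the A button recenters it.
; Its flipbook tracks the character's PullPower, scrubbing Charging until full, then showing Charged.
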(event EventBeginPlay)

(event Collision|EventActorBeginOverlap
  (params (OtherActor :type Actor%20Object%20Reference)))

(event EventTick
  (params (DeltaSeconds :type Float%20%28single-precision%29))
  ;[1 1 1] Wiiリモコン初期設定
  (bind _done (CallFunction|WiiRemoteInitialSetting))
  (if _done
    ;[1 1 1] MotionPlusの値から移動方向を確認し移動量をセットする
    (bind _bmoveup (CallFunction|MoveUp))
    (if _bmoveup
      _
      (else
        (bind _bmovedown (CallFunction|MoveDown))
        (if _bmovedown
          _
          (else
            (Variables|Default|SetmoveZAxisValue 0.0)))))
    (bind _bmoverigth (CallFunction|MoveRight))
    (if _bmoverigth
      _
      (else
        (bind _bmoveleft (CallFunction|MoveLeft))
        (if _bmoveleft
          _
          (else
            (Variables|Default|SetmoveYAxisValue 0.0)))))
    (CallFunction|AimRotate)
    (CallFunction|AimAnim)
    ;[1 1 1] Aボタンが押されたら移動総量をリセット
    (if (Variables|Default|GetbPushAbutton)
      (Utilities|FlowControl|DoOnce false :!label _label
        (:Completed
          (CallFunction|ResetPlayerPitch)))
      (else
        (goto _label Reset)))))

(fn ConstructionScript
  (bind _fpscharacter (Variables|Default|GetfpsCharacter))
  (bind _firstpersoncamera (Variables|/Game/Game/Blueprints/FirstPersonCharacterBP.FirstPersonCharacterBP_C|GetFirstPersonCamera _fpscharacter))
  (Transformation|SetActorLocation (+ (Transformation|GetWorldLocation _firstpersoncamera) (* (Math|Vector|GetForwardVector _firstpersoncamera) (Variables|Default|Getdistance))) false)
  (Transformation|SetActorRotation (Math|Rotator|FindLookatRotation (Transformation|GetActorLocation) (Transformation|GetWorldLocation (Variables|/Game/Game/Blueprints/FirstPersonCharacterBP.FirstPersonCharacterBP_C|GetFirstPersonCamera (Variables|Default|GetfpsCharacter))))))

(fn MoveUp
  (bind _motionpluspitch (Variables|Default|GetmotionPlusPitch))
  (bind _moveupthreshold (Variables|Default|GetmoveUpThreshold))
  (bind _returnvalue (> _motionpluspitch _moveupthreshold))
  (if _returnvalue
    (Variables|Default|SetmoveZAxisValue (* (* (- (Variables|Default|GetmotionPlusPitch) (Variables|Default|GetstandardPitchValue)) -1.0) (Utilities|Time|GetWorldDeltaSeconds))))
  (return _returnvalue))

(fn MoveDown
  (bind _motionpluspitch (Variables|Default|GetmotionPlusPitch))
  (bind _movedownthreshold (Variables|Default|GetmoveDownThreshold))
  (bind _returnvalue (< _motionpluspitch _movedownthreshold))
  (if _returnvalue
    (Variables|Default|SetmoveZAxisValue (* (* (- (Variables|Default|GetmotionPlusPitch) (Variables|Default|GetstandardPitchValue)) -1.0) (Utilities|Time|GetWorldDeltaSeconds))))
  (return _returnvalue))

(fn MoveRight
  (bind _motionplusroll (Variables|Default|GetmotionPlusRoll))
  (bind _moverightthreshold (Variables|Default|GetmoveRightThreshold))
  (bind _returnvalue (< _motionplusroll _moverightthreshold))
  (if _returnvalue
    (Variables|Default|SetmoveYAxisValue (* (* (- (Variables|Default|GetmotionPlusRoll) (Variables|Default|GetstandardRollValue)) -1.0) (Utilities|Time|GetWorldDeltaSeconds))))
  (return _returnvalue))

(fn MoveLeft
  (bind _motionplusroll (Variables|Default|GetmotionPlusRoll))
  (bind _moveleftthreshold (Variables|Default|GetmoveLeftThreshold))
  (bind _returnvalue (> _motionplusroll _moveleftthreshold))
  (if _returnvalue
    (Variables|Default|SetmoveYAxisValue (* (* (- (Variables|Default|GetmotionPlusRoll) (Variables|Default|GetstandardRollValue)) -1.0) (Utilities|Time|GetWorldDeltaSeconds))))
  (return _returnvalue))

(fn ResetPlayerPitch
  (bind _fpscharacter (Variables|Default|GetfpsCharacter))
  (bind _firstpersoncamera (Variables|/Game/Game/Blueprints/FirstPersonCharacterBP.FirstPersonCharacterBP_C|GetFirstPersonCamera _fpscharacter))
  (Transformation|SetActorLocation (+ (Transformation|GetWorldLocation _firstpersoncamera) (* (Math|Vector|GetForwardVector _firstpersoncamera) (Variables|Default|Getdistance))) false))

(fn WiiRemoteInitialSetting
  (if (== (Variables|Default|GetstandardPitchValue) 0.0)
    (Variables|Default|SetstandardPitchValue (Variables|Default|GetmotionPlusPitch))
    (if (== (Variables|Default|GetstandardRollValue) 0.0)
      (Variables|Default|SetstandardRollValue (Variables|Default|GetmotionPlusRoll))
      (Variables|Default|SetmoveUpThreshold (+ (Variables|Default|GetstandardPitchValue) (Variables|Default|GetjudgePlay)))
      (Variables|Default|SetmoveDownThreshold (+ (Variables|Default|GetstandardPitchValue) (* (Variables|Default|GetjudgePlay) -1.0)))
      (Variables|Default|SetmoveRightThreshold (+ (Variables|Default|GetstandardRollValue) (* (Variables|Default|GetjudgePlay) -1.0)))
      (Variables|Default|SetmoveLeftThreshold (+ (Variables|Default|GetstandardRollValue) (Variables|Default|GetjudgePlay)))))
  (return true))

(fn AimRotate
  (bind _fpscharacter (Variables|Default|GetfpsCharacter))
  (bind _firstpersoncamera (Variables|/Game/Game/Blueprints/FirstPersonCharacterBP.FirstPersonCharacterBP_C|GetFirstPersonCamera _fpscharacter))
  (bind _returnvalue (Transformation|GetWorldLocation _firstpersoncamera))
  (Transformation|SetActorRotation (Math|Rotator|FindLookatRotation (Transformation|GetActorLocation) (Transformation|GetWorldLocation (Variables|/Game/Game/Blueprints/FirstPersonCharacterBP.FirstPersonCharacterBP_C|GetFirstPersonCamera (Variables|Default|GetfpsCharacter)))))
  (Transformation|SetActorLocation (+ (* (Math|Vector|Normalize (- (Transformation|GetActorLocation) _returnvalue)) (Variables|Default|Getdistance)) _returnvalue) false)
  (Transformation|AddActorLocalOffset (Math|Vector|MakeVector 0.0 (* (Variables|Default|GetmoveYAxisValue) (Variables|Default|GethorizontalAimSpeed) -1.0) (* (Variables|Default|GetmoveZAxisValue) (Variables|Default|GetverticalAimSpeed) -1.0)) false))

(fn AimAnim
  (bind _fpscharacter (Variables|Default|GetfpsCharacter))
  (bind _fpscharacter_2 (Variables|Default|GetfpsCharacter))
  (bind _aimflipbook (Variables|Default|GetAimFlipBook))
  (if (>= (Variables|/Game/Game/Blueprints/FirstPersonCharacterBP.FirstPersonCharacterBP_C|GetpullPower _fpscharacter_2) (Variables|/Game/Game/Blueprints/FirstPersonCharacterBP.FirstPersonCharacterBP_C|GetmaxPullPower _fpscharacter_2))
    (if (not (== (Class|PaperFlipbookComponent|GetFlipbook (Variables|Default|GetAimFlipBook)) "/Game/Game/Flipbooks/Charged/Charged.Charged"))
      (Sprite|SetFlipbook _aimflipbook "/Game/Game/Flipbooks/Charged/Charged.Charged"))
    (elif (== (Class|PaperFlipbookComponent|GetFlipbook (Variables|Default|GetAimFlipBook)) "/Game/Game/Flipbooks/Charging/Charging.Charging")
      (Components|Timeline|SetNewTime _aimflipbook (* (Class|PaperFlipbookComponent|GetFlipbookLength (Variables|Default|GetAimFlipBook)) (/ (Variables|/Game/Game/Blueprints/FirstPersonCharacterBP.FirstPersonCharacterBP_C|GetpullPower _fpscharacter) (Variables|/Game/Game/Blueprints/FirstPersonCharacterBP.FirstPersonCharacterBP_C|GetmaxPullPower _fpscharacter))))
      (else
        (Sprite|SetFlipbook _aimflipbook "/Game/Game/Flipbooks/Charging/Charging.Charging")))))
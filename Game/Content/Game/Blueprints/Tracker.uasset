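; Tracker is an actor that chases a Target actor at a speed picked at random from the SpeedSeed range when play begins.
; Each Tick it offsets itself toward the Target without sweeping or delta-time scaling, so speed is per frame.
; When its SearchRange component begins overlapping a Scaffold, it stops and records the real time.
; After more than eight seconds stopped, it rerolls its speed and resumes the chase.
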(event OnComponentBeginOverlap(SearchRange)
  (params (OtherActor :type Actor%20Object%20Reference) (OtherComp :type Primitive%20Component%20Object%20Reference) (OtherBodyIndex :type Integer) (bFromSweep :type Boolean) (SweepResult :type Hit%20Result%20Structure%20%28by%20ref%29))
  (Utilities|Casting|CastToScaffold OtherActor)
  (Variables|Default|Setspeed 0.0)
  (Variables|Default|SethitTime (Utilities|Time|GetRealTimeSeconds)))

(event EventBeginPlay
  (bind _speedseed (Variables|Default|GetspeedSeed))
  (bind (_x _y) (Math|Vector2D|BreakVector2D _speedseed))
  (Variables|Default|Setspeed (Math|Random|RandomFloatinRange _x _y)))

(event EventTick
  (params (DeltaSeconds :type Float%20%28single-precision%29))
  (bind _speedseed (Variables|Default|GetspeedSeed))
  (bind (_x _y) (Math|Vector2D|BreakVector2D _speedseed))
  (Transformation|AddActorWorldOffset (* (Math|Vector|Normalize (- (Transformation|GetActorLocation (Variables|Default|Gettarget)) (Transformation|GetActorLocation))) (Variables|Default|Getspeed)))
  (if (== (Variables|Default|Getspeed) 0.0)
    (if (> (- (Utilities|Time|GetRealTimeSeconds) (Variables|Default|GethitTime)) 8.0)
      (Variables|Default|Setspeed (Math|Random|RandomFloatinRange _x _y)))))

(fn ConstructionScript)
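; Enemy pawn that hands its navigation setup to an EnemyAI controller and provides physics-based movement.
; On BeginPlay it casts its controller to EnemyAI and passes it the NavigationVolume and TargetActor.
; MoveTo pushes the capsule from a home location toward a target by adding physics linear velocity, overwriting it at MaxSpeed along that direction once the current speed reaches that limit.
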(event EventBeginPlay
  (bind _asenemy_ai (Utilities|Casting|CastToEnemyAI (Pawn|GetController)))
  (Variables|/Game/Game/Blueprints/AI/Character/EnemyAI.EnemyAI_C|SetNavigationVolume _asenemy_ai (Variables|Default|GetNavigationVolume))
  (Variables|/Game/Game/Blueprints/AI/Character/EnemyAI.EnemyAI_C|SetTargetActor _asenemy_ai (Variables|Default|GetTargetActor)))

(event Collision|EventActorBeginOverlap
  (params (OtherActor :type Actor%20Object%20Reference)))

(event EventTick
  (params (DeltaSeconds :type Float%20%28single-precision%29)))

(fn ConstructionScript)

(fn Moveto
  (params (TargetLocation :type Vector) (HomeLocation :type Vector) (ScaleValue :type Float%20%28single-precision%29) (MaxSpeed :type Float%20%28single-precision%29))
  (bind _returnvalue (- TargetLocation HomeLocation))
  (bind _capsulecomponent (Variables|Collision|GetCapsuleComponent))
  (bind _returnvalue_2 (Math|Vector|Normalize _returnvalue))
  (bind _returnvalue_3 (Physics|GetPhysicsLinearVelocity _capsulecomponent "None"))
  (if (>= (Math|Vector|VectorLength _returnvalue_3) MaxSpeed)
    (Class|PrimitiveComponent|SetAllPhysicsLinearVelocity _capsulecomponent (* _returnvalue_2 MaxSpeed) false)
    (else
      (Class|PrimitiveComponent|SetAllPhysicsLinearVelocity _capsulecomponent (* _returnvalue_2 ScaleValue) true))))
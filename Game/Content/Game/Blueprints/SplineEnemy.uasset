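; Networked enemy that follows a target spline and explodes when hit by a BPArrow.
; It snaps to the spline start at construction, stays hidden until real time reaches SpawnTime, then the authority advances it along the looping spline by Speed.
; An arrow overlap destroys the arrow, multicasts the explosion effect, frees the EnemyAI controller's attack point and destroys the enemy.
; MoveTo and RotateTo provide steering helpers toward a target location.
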(event OnComponentBeginOverlap(Collision)
  (params (OtherActor :type Actor%20Object%20Reference) (OtherComp :type Primitive%20Component%20Object%20Reference) (OtherBodyIndex :type Integer) (bFromSweep :type Boolean) (SweepResult :type Hit%20Result%20Structure%20%28by%20ref%29))
  (bind _asbparrow (Utilities|Casting|CastToBPArrow OtherActor))
  (Actor|DestroyActor _asbparrow)
  (Actor|Tick|SetActorTickEnabled false)
  (CallFunction|Explosion)
  (Utilities|FlowControl|Delay 0.1)
  (bind _asenemy_ai (Utilities|Casting|CastToEnemyAI (Pawn|GetController))
    (:then
      (Variables|/Game/Game/Blueprints/AI/NavigationAI/AttackPointComponent.AttackPointComponent_C|SetIsUsing (Variables|/Game/Game/Blueprints/AI/CharacterAI/EnemyAI.EnemyAI_C|GetAttackPoint _asenemy_ai) false))
    (:CastFailed
      _))
  (Actor|DestroyActor))

(event Custom|ExplosionMulticast
  (Effects|SpawnEmitteratLocation "/Game/StarterContent/Particles/P_Explosion.P_Explosion" (Transformation|GetActorLocation)))

(event Custom|Explosion
  (CallFunction|ExplosionMulticast))

(event EventTick
  (params (DeltaSeconds :type Float%20%28single-precision%29))
  (if (>= (Utilities|Time|GetRealTimeSeconds) (Variables|Default|GetSpawnTime))
    (Rendering|SetVisibility (Variables|Default|GetSkeletalMesh) true false)
    (Networking|SwitchHasAuthority
      (:Authority
        (if (> (Variables|Default|GetSpeed) 0.0)
          (Variables|Default|SetMoveDistance (+ (Variables|Default|GetMoveDistance) (* DeltaSeconds (Variables|Default|GetSpeed))))
          (else
            (Variables|Default|SetMoveDistance (+ (Spline|GetSplineLength (Variables|/Game/Game/Blueprints/SplineActor.SplineActor_C|GetSpline (Variables|Default|GetTargetSpline))) (+ (Variables|Default|GetMoveDistance) (* DeltaSeconds (Variables|Default|GetSpeed)))))))
        (bind (_location _direction _rotation) (Default|GetCurrentLocationandRotation (Variables|Default|GetTargetSpline) (Variables|Default|GetMoveDistance) true))
        (Transformation|SetActorLocation _location false)
        (Transformation|SetActorRotation _rotation)))))

(event EventBeginPlay
  (Rendering|SetVisibility (Variables|Default|GetSkeletalMesh) false false))

(fn ConstructionScript
  (bind _targetspline (Variables|Default|GetTargetSpline))
  (if (Utilities|IsValid _targetspline)
    (bind (_location _direction _rotation) (Default|GetCurrentLocationandRotation _targetspline 0.0 true))
    (Transformation|SetActorLocation _location false)
    (Transformation|SetActorRotation _rotation)))

(fn Moveto
  (params (TargetLocation :type Vector) (ScaleValue :type Float%20%28single-precision%29))
  (Pawn|Input|AddMovementInput (Math|Vector|Normalize (- TargetLocation (Transformation|GetActorLocation))) ScaleValue true))

(fn Rotateto
  (params (TargetLocation :type Vector))
  (Transformation|SetActorRotation (Math|Rotator|Lerp(Rotator) (Transformation|GetActorRotation) (Math|Rotator|FindLookatRotation (Transformation|GetActorLocation) TargetLocation) 0.1)))
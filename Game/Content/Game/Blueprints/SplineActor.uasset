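; Spline rail actor that builds a rail mesh along its spline and exposes helpers for querying positions along that path.
; The construction script labels each spline point with its index using text hidden in game, and pads a per-segment Visible array with true.
; It adds a RailMesh spline mesh for each visible segment, so sections can be omitted.
; Functions return location, direction and rotation at a distance with optional looping, and report end-of-spline arrival.
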(event EventBeginPlay)

(event Collision|EventActorBeginOverlap
  (params (OtherActor :type Actor%20Object%20Reference)))

(event EventTick
  (params (DeltaSeconds :type Float%20%28single-precision%29)))

(fn ConstructionScript
  (bind _spline (Variables|Default|GetSpline))
  ;[1 1 1] 制御点のインデックスを表示させる
  (for _index (range 0 (- (Class|SplineComponent|GetNumSplinePoints (Variables|Default|GetSpline)) 1))
    (bind _rotation (CallFunction|GetCurrentLocationandRotation (Spline|GetDistanceAlongSplineatSplinePoint (Variables|Default|GetSpline) _index) false))
    (bind _returnvalue (AddComponent|AddTextRenderComponent false (Math|Transform|MakeTransform (.LocalLocation (Class|SplineComponent|GetLocalLocationandTangentatSplinePoint (Variables|Default|GetSpline) _index)) _rotation)))
    (Rendering|Components|TextRender|SetText _returnvalue (Utilities|Text|ToText(Integer) _index))
    (Rendering|Components|TextRender|SetXScale _returnvalue 3.0)
    (Rendering|Components|TextRender|SetYScale _returnvalue 3.0)
    (Development|SetHiddeninGame _returnvalue true false)
    (if (< (Utilities|Array|Length (Variables|Default|GetbVisible)) (- (Class|SplineComponent|GetNumSplinePoints (Variables|Default|GetSpline)) 1))
      (Utilities|Array|Add (Variables|Default|GetbVisible) true)))
  ;[1 1 1] splineに沿ったメッシュ作成
  (for _index_2 (range 0 (- (Class|SplineComponent|GetNumSplinePoints (Variables|Default|GetSpline)) 2))
    (if (Utilities|Array|Get(acopy) (Variables|Default|GetbVisible) _index_2)
      (bind _returnvalue_2 (AddComponent|AddSplineMeshComponent false))
      (Components|StaticMesh|SetStaticMesh _returnvalue_2 (Variables|Default|GetrailMesh))
      (SplineMesh|SetStartandEnd _returnvalue_2 (.LocalLocation (Class|SplineComponent|GetLocalLocationandTangentatSplinePoint _spline _index_2)) (.LocalTangent (Class|SplineComponent|GetLocalLocationandTangentatSplinePoint _spline _index_2)) (.LocalLocation (Class|SplineComponent|GetLocalLocationandTangentatSplinePoint _spline (+ _index_2 1))) (.LocalTangent (Class|SplineComponent|GetLocalLocationandTangentatSplinePoint _spline (+ _index_2 1))) :!class /Script/Engine.SplineMeshComponent))))

(fn GetCurrentLocationandRotation
  (params (Length :type Float%20%28single-precision%29) (Loop :type Boolean))
  (bind _spline (Variables|Default|GetSpline))
  (if Loop
    (LocalVariables|SetLocalLength (Math|Float|%(Float) Length (Spline|GetSplineLength (Variables|Default|GetSpline))))
    (else
      (LocalVariables|SetLocalLength Length)))
  (return (Class|SplineComponent|GetWorldLocationatDistanceAlongSpline _spline (LocalVariables|GetLocalLength)) (Class|SplineComponent|GetWorldDirectionatDistanceAlongSpline _spline (LocalVariables|GetLocalLength)) (Class|SplineComponent|GetWorldRotationatDistanceAlongSpline _spline (LocalVariables|GetLocalLength))))

(fn IsArrived
  (params (Length :type Float%20%28single-precision%29))
  (return (>= Length (Spline|GetSplineLength (Variables|Default|GetSpline)))))
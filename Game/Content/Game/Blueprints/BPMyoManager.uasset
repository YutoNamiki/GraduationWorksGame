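; BPMyoManager is a Myo armband controller that fires bow arrows by hand gesture.
; On Tick, when the pull and shoot flags are both set, it first vibrates the armband once as a ready cue.
; A fingers-spread pose then spawns a BPArrow at the manager's transform and launches it along local X.
; Firing vibrates again and clears the state flags and stored fist acceleration.
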(event EventBeginPlay)

(event Collision|EventActorBeginOverlap
  (params (OtherActor :type Actor%20Object%20Reference)))

(event EventTick
  (params (DeltaSeconds :type Float%20%28single-precision%29))
  (if (Variables|Default|GetbCanPullString)
    (if (Variables|Default|GetbCanShootArrow)
      (if (Variables|Default|Getvibrate)
        (if (Variables|Default|GetbMyoPoseFingersSpread)
          (bind _returnvalue (Game|SpawnActorfromClass "/Game/Game/Maps/Takemura/BPArrow.BPArrow_C" (Transformation|GetActorTransform) false 0 0))
          (bind _output_get (Variables|Default|SetbpArrow _returnvalue))
          (Game|Components|ProjectileMovement|SetVelocityinLocalSpace (Actor|GetComponentsByClass _output_get "/Script/Engine.ProjectileMovementComponent") "2000.000000, 0, 0")
          (Variables|Default|SetbCanShootArrow false)
          (Variables|Default|SetbCanPullString false)
          (Variables|Default|Setvibrate false)
          (Variables|Default|SetaccelXatFist 0.0)
          (Class|TestMyoPawn|MyoVibrate))
        (else
          (Class|TestMyoPawn|MyoVibrate)
          (Variables|Default|Setvibrate true))))))

(fn ConstructionScript)
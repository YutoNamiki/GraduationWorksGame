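; Scaffold is a moving platform that rides a referenced spline in a loop, starting at StartLength and playing a sound on BeginPlay.
; Tick advances distance by Speed, derives the lap count and snaps location and rotation to the spline.
; Overlapping a TramSpeedChanger replaces Speed once its lap threshold is reached.
; It also collects its AttackPointComponents and reserves the nearest free one on request, though the first is the default even if occupied.
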(event OnComponentBeginOverlap(Sphere)
  (params (OtherActor :type Actor%20Object%20Reference) (OtherComp :type Primitive%20Component%20Object%20Reference) (OtherBodyIndex :type Integer) (bFromSweep :type Boolean) (SweepResult :type Hit%20Result%20Structure%20%28by%20ref%29))
  (bind _astram_speed_changer (Utilities|Casting|CastToTramSpeedChanger OtherActor))
  (if (>= (Variables|Default|GetLap) (- (Variables|/Game/Game/Blueprints/TramSpeedChanger.TramSpeedChanger_C|GetTargetLap _astram_speed_changer) 1))
    (Variables|Default|SetSpeed (Variables|/Game/Game/Blueprints/TramSpeedChanger.TramSpeedChanger_C|GetChangeSpeed _astram_speed_changer))))

(event EventTick
  (params (DeltaSeconds :type Float%20%28single-precision%29))
  (Networking|SwitchHasAuthority
    (:Authority
      _)
    (:Remote
      _))
  (if (> (Variables|Default|GetSpeed) 0.0)
    (Variables|Default|SetMoveDistance (+ (Variables|Default|GetMoveDistance) (* DeltaSeconds (Variables|Default|GetSpeed))))
    (else
      (Variables|Default|SetMoveDistance (+ (Spline|GetSplineLength (Variables|/Game/Game/Blueprints/SplineActor.SplineActor_C|GetSpline (Variables|Default|GetSpline))) (+ (Variables|Default|GetMoveDistance) (* DeltaSeconds (Variables|Default|GetSpeed)))))))
  (Variables|Default|SetLap (Math|Float|Truncate (/ (Variables|Default|GetMoveDistance) (Spline|GetSplineLength (Variables|/Game/Game/Blueprints/SplineActor.SplineActor_C|GetSpline (Variables|Default|GetSpline))))))
  (bind (_location _direction _rotation) (Default|GetCurrentLocationandRotation (Variables|Default|GetSpline) (Variables|Default|GetMoveDistance) true))
  (Transformation|SetActorLocation _location false)
  (Transformation|SetActorRotation _rotation))

(event EventBeginPlay
  (Audio|PlaySoundatLocation "/Game/Game/Sounds/SE/Tram/gotogoto.gotogoto" (Transformation|GetActorLocation)))

(fn ConstructionScript
  (bind _startlength (Variables|Default|GetStartLength))
  (Variables|Default|SetMoveDistance _startlength)
  (bind (_location _direction _rotation) (Default|GetCurrentLocationandRotation (Variables|Default|GetSpline) _startlength true))
  (Transformation|SetActorLocation _location false)
  (Transformation|SetActorRotation _rotation)
  (Utilities|Array|Clear (Variables|Default|GetAttackPoints))
  (Variables|Default|SetAttackPoints (Actor|GetComponentsByClass "/Game/Game/Blueprints/AI/NavigationAI/AttackPointComponent.AttackPointComponent_C")))

(fn GetNearestUseableAttackPoint
  (params (CurrentLocation :type Vector))
  (bind _attackpoints (Variables|Default|GetAttackPoints))
  (LocalVariables|SetCurrent CurrentLocation)
  (LocalVariables|SetNearestAttackPoint (Utilities|Array|Get(acopy) _attackpoints))
  (for _index (range 1 (Utilities|Array|LastIndex _attackpoints))
    (if (not (Variables|/Game/Game/Blueprints/AI/NavigationAI/AttackPointComponent.AttackPointComponent_C|GetIsUsing (Utilities|Array|Get(acopy) _attackpoints _index)))
      (if (< (Math|Vector|VectorLength (- (LocalVariables|GetCurrent) (Transformation|GetWorldLocation (Utilities|Array|Get(acopy) _attackpoints _index)))) (Math|Vector|VectorLength (- (LocalVariables|GetCurrent) (Transformation|GetWorldLocation (LocalVariables|GetNearestAttackPoint)))))
        (LocalVariables|SetNearestAttackPoint (Utilities|Array|Get(acopy) _attackpoints _index)))))
  (Variables|/Game/Game/Blueprints/AI/NavigationAI/AttackPointComponent.AttackPointComponent_C|SetIsUsing (LocalVariables|GetNearestAttackPoint) true)
  (return (LocalVariables|GetNearestAttackPoint)))
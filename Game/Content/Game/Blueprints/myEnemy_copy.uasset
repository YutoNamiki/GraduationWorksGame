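; Enemy actor that patrols a looping spline at a random speed and direction, and can break off to chase the player.
; When a Scaffold's sphere enters SearchRange, a random roll may switch Tick from spline movement to homing on the Target's PlayerPosition.
; Overlap of Sphere1 with a Scaffold's sphere or a BPArrow spawns an explosion and destroys the enemy.
; The construction script snaps it to the first spline point.
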(event OnComponentBeginOverlap(Sphere1)
  (params (OtherActor :type Actor%20Object%20Reference) (OtherComp :type Primitive%20Component%20Object%20Reference) (OtherBodyIndex :type Integer) (bFromSweep :type Boolean) (SweepResult :type Hit%20Result%20Structure%20%28by%20ref%29))
  (bind _asscaffold (Utilities|Casting|CastToScaffold OtherActor)
    (:then
      (if (== (Variables|/Game/Game/Blueprints/Scaffold.Scaffold_C|GetSphere _asscaffold) OtherComp)
        (Effects|SpawnEmitteratLocation "/Game/StarterContent/Particles/P_Explosion.P_Explosion" (Transformation|GetActorLocation) :!label _label)
        (Actor|DestroyActor)))
    (:CastFailed
      (Utilities|Casting|CastToBPArrow OtherActor)
      (goto _label))))

(event OnComponentHit(Sphere1)
  (params (OtherActor :type Actor%20Object%20Reference) (OtherComp :type Primitive%20Component%20Object%20Reference) (NormalImpulse :type Vector :default "0, 0, 0") (Hit :type Hit%20Result%20Structure%20%28by%20ref%29)))

(event OnComponentBeginOverlap(SearchRange)
  (params (OtherActor :type Actor%20Object%20Reference) (OtherComp :type Primitive%20Component%20Object%20Reference) (OtherBodyIndex :type Integer) (bFromSweep :type Boolean) (SweepResult :type Hit%20Result%20Structure%20%28by%20ref%29))
  (bind _asscaffold (Utilities|Casting|CastToScaffold OtherActor))
  (if (== (Variables|/Game/Game/Blueprints/Scaffold.Scaffold_C|GetSphere _asscaffold) OtherComp)
    (if (> (Math|Random|RandomIntegerinRange -3 8) 0)
      (Variables|Default|SetsetTarget true))))

(event EventBeginPlay
  (bind _speedseedplus (Variables|Default|GetspeedSeedPlus))
  (bind _speedseedminus (Variables|Default|GetspeedSeedMinus))
  (bind (_x _y) (Math|Vector2D|BreakVector2D _speedseedminus))
  (bind (_x_2 _y_2) (Math|Vector2D|BreakVector2D _speedseedplus))
  (if (> (Math|Random|RandomFloatinRange -8e+01 8e+01) 0.0)
    (Variables|Default|Setspeed (Math|Random|RandomFloatinRange _x_2 _y_2))
    (else
      (Variables|Default|Setspeed (Math|Random|RandomFloatinRange _x _y)))))

(event Collision|EventActorBeginOverlap
  (params (OtherActor :type Actor%20Object%20Reference)))

(event EventTick
  (params (DeltaSeconds :type Float%20%28single-precision%29))
  (if (Variables|Default|GetsetTarget)
    (Transformation|AddActorWorldOffset (* (Math|Vector|Normalize (- (Transformation|GetWorldLocation (Variables|/Game/Game/Blueprints/Scaffold.Scaffold_C|GetplayerPosition (Variables|Default|Gettarget))) (Transformation|GetActorLocation))) (Variables|Default|GettoTargetSpeed)))
    (else
      (if (> (Variables|UserOptions|Basic|GetSpeed) 0.0)
        (Variables|Default|SetMoveDistance (+ (Variables|Default|GetMoveDistance) (* DeltaSeconds (Variables|UserOptions|Basic|GetSpeed))))
        (else
          (Variables|Default|SetMoveDistance (+ (Spline|GetSplineLength (Variables|/Game/Game/Blueprints/SplineActor.SplineActor_C|GetSpline (Variables|Components|GetSpline))) (+ (Variables|Default|GetMoveDistance) (* DeltaSeconds (Variables|UserOptions|Basic|GetSpeed)))))))
      (bind _location (Default|GetCurrentLocationandRotation (Variables|Components|GetSpline) (Variables|Default|GetMoveDistance) true))
      (Transformation|SetActorLocation _location false))))

(fn ConstructionScript
  (Transformation|SetActorLocation (Class|SplineComponent|GetWorldLocationatSplinePoint (Variables|/Game/Game/Blueprints/SplineActor.SplineActor_C|GetSpline (Variables|Default|Getspline))) false))